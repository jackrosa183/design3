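; BP_PathPickup is a pickup that raises a referenced bridge part when a capsule component overlaps its cube.
; The overlap calls MoveBridge, hides the cube without disabling its collision, and plays a 2D robot sound.
; MoveBridge plays a timeline that lerps the bridge from its current location toward one unit higher on every update, so the total rise accumulates per frame instead of reaching a fixed target.
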(event OnComponentBeginOverlap(Cube)
  (params (OverlappedComponent :type Primitive%20Component%20Object%20Reference) (OtherActor :type Actor%20Object%20Reference) (OtherComp :type Primitive%20Component%20Object%20Reference) (OtherBodyIndex :type Integer) (bFromSweep :type Boolean) (SweepResult :type Hit%20Result%20Structure%20%28by%20ref%29))
  (Utilities|Casting|CastToCapsuleComponent OtherComp)
  (CallFunction|MoveBridge)
  (Development|SetHiddeninGame (Variables|Default|GetCube) true false)
  (Audio|PlaySound2D "/Game/Sound/robotsound3.robotsound3" 1.0 1.0 0.0 0 0))

(event Custom|MoveBridge
  (bind _bridge_part (Variables|Default|GetBridge_Part))
  (bind _rootcomponent (Variables|/Script/Engine.Actor|GetRootComponent _bridge_part))
  (bind _returnvalue (Transformation|GetWorldLocation _rootcomponent))
  (bind _newtrack_0 (Timeline|Timeline_0 Play)
    (:Update
      (Transformation|SetWorldLocation (Variables|/Script/Engine.StaticMeshActor|GetStaticMeshComponent _bridge_part) (Math|Vector|Lerp(Vector) (Transformation|GetWorldLocation _rootcomponent) (Math|Vector|MakeVector (.x _returnvalue) (.y _returnvalue) (+ (.z _returnvalue) 1.0)) _newtrack_0) false false))))

(fn ConstructionScript)