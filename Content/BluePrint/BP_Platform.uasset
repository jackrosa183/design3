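; Moving platform actor that travels along a referenced spline path and can optionally show a ramp mesh or collapse when fragile.
; Timelines drive its position and rotation: Timeline_0 starts automatically if AlwaysMoving, otherwise MoveTowardsPlayer plays MoveTimeLIne at a PathSpeed-based rate.
; Leaving Light_Trigger while the character's HittingReceiver is set stops on-demand movement.
; Standing on a fragile platform makes its pieces fall with physics after DurabiltyTime, then destroys them.
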(event OnComponentBeginOverlap(Surface_Collider)
  (params (OverlappedComponent :type Primitive%20Component%20Object%20Reference) (OtherActor :type Actor%20Object%20Reference) (OtherComp :type Primitive%20Component%20Object%20Reference) (OtherBodyIndex :type Integer) (bFromSweep :type Boolean) (SweepResult :type Hit%20Result%20Structure%20%28by%20ref%29))
  (bind _asfirst_person_character (Utilities|Casting|CastToFirstPersonCharacter OtherActor))
  (if (Variables|/Game/FirstPersonBP/Blueprints/FirstPersonCharacter.FirstPersonCharacter_C|GetisOnPlatform? _asfirst_person_character)
    (Variables|Default|SetisStandingOn? true)
    (if (Variables|Default|GetisFragile?)
      (Utilities|FlowControl|Delay (Math|Conversions|ToFloat(Integer) (Variables|Default|GetDurabilty_Time)))
      (if (Variables|Default|GetisStandingOn?)
        (Utilities|FlowControl|Sequence
          (:then_0
            (Physics|SetSimulatePhysics (Variables|Default|GetCone%28replace%29) true))
          (:then_1
            (Physics|SetSimulatePhysics (Variables|Default|GetReplace) true)
            (Utilities|FlowControl|Delay 3.0)
            (Components|DestroyComponent (Variables|Default|GetReplace))
            (Components|DestroyComponent (Variables|Default|GetCone%28replace%29))))))))

(event OnComponentEndOverlap(Light_Trigger)
  (params (OverlappedComponent :type Primitive%20Component%20Object%20Reference) (OtherActor :type Actor%20Object%20Reference) (OtherComp :type Primitive%20Component%20Object%20Reference) (OtherBodyIndex :type Integer))
  (bind _path (Variables|Default|GetPath))
  (bind _path_spline (Variables|/Game/BluePrint/BP_Path.BP_Path_C|GetPath_Spline _path))
  (bind _asfirst_person_character (Utilities|Casting|CastToFirstPersonCharacter OtherActor))
  (if (Variables|/Game/FirstPersonBP/Blueprints/FirstPersonCharacter.FirstPersonCharacter_C|GethittingReceiver? _asfirst_person_character)
    (if (not (Variables|Default|GetalwaysMoving?))
      (bind _path_alpha (Timeline|MoveTimeLIne Stop)
        (:Update
          (Variables|Default|SetPath%20Alpha _path_alpha)
          (Transformation|SetActorLocationAndRotation (Spline|GetLocationatDistanceAlongSpline _path_spline (Math|Float|Lerp 0.0 (Spline|GetSplineLength _path_spline) (Variables|Default|GetPath%20Alpha)) "World") (Spline|GetRotationatDistanceAlongSpline _path_spline (Math|Float|Lerp 0.0 (Spline|GetSplineLength _path_spline) (Variables|Default|GetPath%20Alpha)) "Local")))))))

(event Custom|MoveTowardsPlayer
  (bind _path (Variables|Default|GetPath))
  (bind _path_spline (Variables|/Game/BluePrint/BP_Path.BP_Path_C|GetPath_Spline _path))
  (if (not (Variables|Default|GetalwaysMoving?))
    (Components|Timeline|SetPlayRate (Variables|Default|GetMoveTimeLIne) (/ 1.0 (Variables|Default|GetPathSpeed)))
    (bind _path_alpha (Timeline|MoveTimeLIne Play)
      (:Update
        (Variables|Default|SetPath%20Alpha _path_alpha)
        (Transformation|SetActorLocationAndRotation (Spline|GetLocationatDistanceAlongSpline _path_spline (Math|Float|Lerp 0.0 (Spline|GetSplineLength _path_spline) (Variables|Default|GetPath%20Alpha)) "World") (Spline|GetRotationatDistanceAlongSpline _path_spline (Math|Float|Lerp 0.0 (Spline|GetSplineLength _path_spline) (Variables|Default|GetPath%20Alpha)) "Local"))))))

(event Custom|StopMoving
  (bind _path (Variables|Default|GetPath))
  (bind _path_2 (Variables|Default|GetPath))
  (bind _path_spline (Variables|/Game/BluePrint/BP_Path.BP_Path_C|GetPath_Spline _path))
  (bind _path_spline_2 (Variables|/Game/BluePrint/BP_Path.BP_Path_C|GetPath_Spline _path_2))
  (if (Variables|Default|GetalwaysMoving?)
    (bind _path_alpha (Timeline|Timeline_0 Stop)
      (:Update
        (Variables|Default|SetPath%20Alpha _path_alpha)
        (Transformation|SetActorLocationAndRotation (Spline|GetLocationatDistanceAlongSpline _path_spline_2 (Math|Float|Lerp 0.0 (Spline|GetSplineLength _path_spline_2) (Variables|Default|GetPath%20Alpha)) "World") (Spline|GetRotationatDistanceAlongSpline _path_spline_2 (Math|Float|Lerp 0.0 (Spline|GetSplineLength _path_spline_2) (Variables|Default|GetPath%20Alpha)) "Local"))))
    (else
      (bind _path_alpha_2 (Timeline|MoveTimeLIne Stop)
        (:Update
          (Variables|Default|SetPath%20Alpha _path_alpha_2)
          (Transformation|SetActorLocationAndRotation (Spline|GetLocationatDistanceAlongSpline _path_spline (Math|Float|Lerp 0.0 (Spline|GetSplineLength _path_spline) (Variables|Default|GetPath%20Alpha)) "World") (Spline|GetRotationatDistanceAlongSpline _path_spline (Math|Float|Lerp 0.0 (Spline|GetSplineLength _path_spline) (Variables|Default|GetPath%20Alpha)) "Local")))))))

(event Custom|Play
  (bind _path (Variables|Default|GetPath))
  (bind _path_spline (Variables|/Game/BluePrint/BP_Path.BP_Path_C|GetPath_Spline _path))
  (bind _path_alpha (Timeline|Timeline_0 Play)
    (:Update
      (Variables|Default|SetPath%20Alpha _path_alpha)
      (Transformation|SetActorLocationAndRotation (Spline|GetLocationatDistanceAlongSpline _path_spline (Math|Float|Lerp 0.0 (Spline|GetSplineLength _path_spline) (Variables|Default|GetPath%20Alpha)) "World") (Spline|GetRotationatDistanceAlongSpline _path_spline (Math|Float|Lerp 0.0 (Spline|GetSplineLength _path_spline) (Variables|Default|GetPath%20Alpha)) "Local")))))

(event Custom|LoopMovement
  (bind _path (Variables|Default|GetPath))
  (bind _path_spline (Variables|/Game/BluePrint/BP_Path.BP_Path_C|GetPath_Spline _path))
  (Components|Timeline|SetPlayRate (Variables|Default|GetMoveTimeLIne) (/ 1.0 (Variables|Default|GetPathSpeed)))
  (bind _path_alpha (Timeline|Timeline_0 Play)
    (:Update
      (Variables|Default|SetPath%20Alpha _path_alpha)
      (Transformation|SetActorLocationAndRotation (Spline|GetLocationatDistanceAlongSpline _path_spline (Math|Float|Lerp 0.0 (Spline|GetSplineLength _path_spline) (Variables|Default|GetPath%20Alpha)) "World") (Spline|GetRotationatDistanceAlongSpline _path_spline (Math|Float|Lerp 0.0 (Spline|GetSplineLength _path_spline) (Variables|Default|GetPath%20Alpha)) "Local")))))

(event EventBeginPlay
  (Utilities|FlowControl|Sequence
    (:then_0
      (if (Variables|Default|GethasRamp?)
        (Components|StaticMesh|SetStaticMesh (Variables|Default|GetRamp_Component) (Variables|Default|GetRampMesh))))
    (:then_1
      (if (Variables|Default|GetalwaysMoving?)
        (CallFunction|LoopMovement)))))

(fn ConstructionScript)